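; MonsterBP is a horror monster actor that rotates to face the player every tick and tracks a target distance.
; BeginPlay caches the player pawn and its movement component, and Sprint input events set a sprinting flag.
; Tick raises TargetDistance over time while the player sprints on the ground and lowers it whenever the player is off the ground.
; Nothing in these graphs applies TargetDistance to the monster's position.
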(event EventBeginPlay
  (bind _returnvalue (Game|Player|GetPlayerPawn 0))
  ;[1 1 1] Get References to Player
  (Variables|Default|SetPlayer _returnvalue)
  (bind _ascharacter (Utilities|Casting|CastToCharacter _returnvalue)
    (:then
      (Variables|Default|SetPlayerMovement (Pawn|GetMovementComponent _ascharacter)))
    (:CastFailed
      (Development|PrintString "ERROR: Player isn't a Pawn!" true true "(R=1.000000,G=1.000000,B=1.000000,A=1.000000)"))))

(event EventTick
  (params (DeltaSeconds :type Float%20%28single-precision%29))
  ;[1 1 1] Update Logic
  (Utilities|FlowControl|Sequence
    (:then_0
      ;;[1 1 1] Rotate to Face Player
      (Transformation|SetActorRotation (Math|Rotator|FindLookatRotation (Transformation|GetActorLocation) (Transformation|GetActorLocation (Variables|Default|GetPlayer)))))
    (:then_1
      ;;[1 1 1] Update Target Distance
      (if (AI|Components|NavMovement|IsMovingonGround (Variables|Default|GetPlayerMovement))
        (if (Variables|Monster|GetIsPlayerSprinting?)
          (Variables|Monster|SetTargetDistance (+ (Variables|Monster|GetTargetDistance) (* DeltaSeconds (Variables|Monster|GetTargetDistanceIncreaseRate)))))
        (else
          (Variables|Monster|SetTargetDistance (- (Variables|Monster|GetTargetDistance) (* DeltaSeconds (Variables|Monster|GetTargetDistanceIncreaseRate)))))))))

(event Input|ActionEvents|InputActionSprint
  ;[1 1 1] Track Player Sprinting
  (:Pressed
    (Variables|Monster|SetIsPlayerSprinting? true))
  (:Released
    (Variables|Monster|SetIsPlayerSprinting? false)))

(fn ConstructionScript)