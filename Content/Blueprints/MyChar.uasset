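; Player character Blueprint that provides basic mouse look and WASD movement.
; Mouse axis events drive controller yaw and inverted-sign pitch.
; Tick polls W, S, D and A directly on player controller 0 instead of using input mappings for movement.
; Each held key adds reduced-scale movement input along the actor's forward or right vector, flattened to horizontal and normalized, negated for backward and left.
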(event EventTick
  (params (DeltaSeconds :type Float%20%28single-precision%29))
  (bind _returnvalue (Game|GetPlayerController 0))
  (bind _self self)
  (bind _returnvalue_2 (Transformation|GetActorForwardVector _self))
  (bind _returnvalue_3 (Transformation|GetActorRightVector _self))
  (bind (_x _y) (Math|Vector|BreakVector _returnvalue_2))
  (bind (_x_2 _y_2) (Math|Vector|BreakVector _returnvalue_3))
  (bind _returnvalue_4 (Math|Vector|MakeVector _x _y 0.0))
  (bind _returnvalue_5 (Math|Vector|MakeVector _x_2 _y_2 0.0))
  (bind _returnvalue_6 (Math|Vector|Normalize _returnvalue_4))
  (bind _returnvalue_7 (Math|Vector|Normalize _returnvalue_5))
  (Utilities|FlowControl|Sequence
    (:then_0
      ;[1 1 1] Forward/Backward Movement Input
      (if (Game|Player|IsInputKeyDown _returnvalue "W")
        (Pawn|Input|AddMovementInput _returnvalue_6 0.475)))
    (:then_1
      (if (Game|Player|IsInputKeyDown _returnvalue "S")
        (Pawn|Input|AddMovementInput (Math|Vector|NegateVector _returnvalue_6) 0.475)))
    (:then_2
      ;[1 1 1] Left/Right Movement Input
      (if (Game|Player|IsInputKeyDown _returnvalue "D")
        (Pawn|Input|AddMovementInput _returnvalue_7 0.475)))
    (:then_3
      (if (Game|Player|IsInputKeyDown _returnvalue "A")
        (Pawn|Input|AddMovementInput (Math|Vector|NegateVector _returnvalue_7) 0.475)))))

(event Input|MouseEvents|MouseX
  (params (AxisValue :type Float%20%28single-precision%29))
  ;[1 1 1] Rotation Input
  (Pawn|Input|AddControllerYawInput (* AxisValue 1.0)))

(event Input|MouseEvents|MouseY
  (params (AxisValue :type Float%20%28single-precision%29))
  ;[1 1 1] Rotation Input
  (Pawn|Input|AddControllerPitchInput (* AxisValue -1.0)))

(fn ConstructionScript)